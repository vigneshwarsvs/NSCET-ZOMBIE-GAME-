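; Zombie enemy that chases the player, attacks in melee and can be killed.
; It loops AI MoveTo toward player controller 0 into an attack montage, whose notify runs a sphere overlap at an arrow to damage the player character.
; Pawn sensing raises its walk speed on sight.
; Point damage reduces health, playing a hit reaction or death, which disables capsule collision, notifies the zombie game mode and destroys it after a delay.
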(event `self.PawnSensing.OnSeePawn`
  (params (Pawn :type "Pawn Object Reference"))
  ;[1 1 1] set
  (set `CharacterMovementComponent.MaxWalkSpeed` 360.0 (`self.CharacterMovement`)))

(event `self.ReceiveBeginPlay`
  ;[1 1 1] event begin
  (`self.runtoplayer`))

(event `runtoplayer`
  ;[1 1 1] chase
  (if (not (`self.isdeath?`))
    (`|AIMoveTo` self (0.0 0.0 0.0) (`GameplayStatics.GetPlayerController` 0) 40.0
      (:`OnSuccess`
        (`self.attackplayer`))
      (:`OnFail`
        (`self.runtoplayer`)))))

(event `attackplayer`
  ;[1 1 1] attack
  (`|PlayMontage` (`self.Mesh`) "/Game/_MAIN/zombie/animations/zombie_attack_Montage1.zombie_attack_Montage1"
    (:`OnCompleted`
      (`self.runtoplayer`))
    (:`OnNotifyBegin`
      (`GameplayStatics.PlaySoundAtLocation` "/Game/_MAIN/zombie/SOUNDS/ATTACKSOUND.ATTACKSOUND" (`self.K2_GetActorLocation`) (struct) 1.0 1.0 0.0 "/Game/MilitaryWeapSilver/Sound/Attenuation/WeaponShot_att.WeaponShot_att" null null null)
      (bind (_outactors _returnvalue) (`KismetSystemLibrary.SphereOverlapActors` (`SceneComponent.K2_GetComponentLocation` (`self.Arrow1`)) 80.0 (`|MakeArray` "ObjectTypeQuery3" :!type "EObjectTypeQuery Enum") "/Game/_MAIN/BLUEPRINTS/BP_FirstPersonCharacter.BP_FirstPersonCharacter_C" (`|MakeArray` self :!type "Actor Object Reference")))
      (if _returnvalue
        (for _array_element _outactors
          (`GameplayStatics.ApplyDamage` _array_element 20.0 (`self.GetController`) self "/Script/Engine.DamageType"))))))

(event `self.ReceivePointDamage`
  (params (Damage :type "Float (single-precision)") (DamageType :type "DamageType Object Reference") (HitLocation :type "Vector Structure") (HitNormal :type "Vector Structure") (HitComponent :type "PrimitiveComponent Object Reference") (BoneName :type Name) (ShotFromDirection :type "Vector Structure") (InstigatedBy :type "Controller Object Reference") (DamageCauser :type "Actor Object Reference") (HitInfo :type "HitResult Structure (by ref)"))
  ;[1 1 1] aplly damage
  (if (`self.isdeath?`)
    _
    (elif (<= (`self.health`) 0.0)
      (`self.death`)
      (else
        (bind _output_get (set `self.health` (- (`self.health`) Damage)))
        (`KismetSystemLibrary.PrintString` (`KismetStringLibrary.Conv_DoubleToString` _output_get))
        (if (<= _output_get 0.0)
          (`self.death`)
          (else
            (`|PlayMontage` (`self.Mesh`) "/Game/_MAIN/zombie/animations/Zombie_Reaction_Hit_mixamo_com_Montage.Zombie_Reaction_Hit_mixamo_com_Montage")))))))

(event `death`
  ;[1 1 1] zombie death
  (set `self.isdeath?` true)
  (`MovementComponent.StopMovementImmediately` (`self.CharacterMovement`))
  (`|PlayMontage` (`self.Mesh`) "/Game/_MAIN/zombie/animations/zombie_dying_Montage.zombie_dying_Montage"
    (:`then`
      (`PrimitiveComponent.SetCollisionEnabled` (`self.CapsuleComponent`) "NoCollision")
      (`PrimitiveComponent.SetCollisionResponseToChannel` (`self.CapsuleComponent`) "ECC_Pawn" "ECR_Overlap")
      (`PrimitiveComponent.SetCollisionResponseToChannel` (`self.Mesh`) "ECC_Pawn" "ECR_Overlap")
      (bind _aszombiegamemode (cast `/Game/_MAIN/BLUEPRINTS/zombiegamemode` (`GameplayStatics.GetGameMode`)))
      (`/Game/_MAIN/BLUEPRINTS/zombiegamemode.ZOMBIEKILLED` _aszombiegamemode)
      (`KismetSystemLibrary.Delay` 10.0)
      (`self.K2_DestroyActor`))))

(fn `UserConstructionScript`)