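; Zombie wave game mode that spawns enemies, tracks kills and ends in a player win after the final wave.
; Each wave sets its kill target from the wave number, then spawns half that count at each of four locations, twice the target in total.
; ZOMBIEKILLED counts down the target and advances the wave at zero.
; Later waves show character UI before a delayed spawn; the last triggers the win UI.
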(event `WAVE START`
  ;[1 1 1] start
  (bind _asbp_first_person_character (cast `/Game/_MAIN/BLUEPRINTS/BP_FirstPersonCharacter` (`GameplayStatics.GetPlayerCharacter` 0)))
  (`/Game/_MAIN/BLUEPRINTS/BP_FirstPersonCharacter.SHOW WAVE UI` _asbp_first_person_character (`self.CURRENT WAVE`))
  (`KismetSystemLibrary.Delay` 5.0)
  (`self.spawn zombie`))

(event `self.ReceiveBeginPlay`
  ;[1 1 1] start game
  (`self.start game`))

(event `start game`
  ;[1 1 1] start game
  (`self.spawn zombie`))

(event `ZOMBIEKILLED`
  ;[1 1 1] ZOMBIE KILLED
  (bind _result (`/Engine/EditorBlueprintResources/StandardMacros.DecrementInt` (`self.ZOMBIES LEFT`))
    (:`  `
      (if (== _result 0)
        (`self.WAVE INCREAMENT`)))))

(event `spawn zombie`
  ;[1 1 1] SPAWN ZOMBIES
  (bind _output_get (set `self.ZOMBIETOTAL` (* (`self.CURRENT WAVE`) 4)))
  (set `self.ZOMBIES LEFT` _output_get)
  (for _index (range (+ _output_get 1))
    (if (== _index (/ (`self.ZOMBIETOTAL`) 2))
      (break)
      (else
        (`|SpawnActorFromClass` "/Game/_MAIN/zombie/bp_zombie.bp_zombie_C" (`self.Spawn LOCATION1`) "Undefined" "OverrideRootScale" null null))))
  (for _ (range 1 (+ (/ (`self.ZOMBIETOTAL`) 2) 1))
    (`|SpawnActorFromClass` "/Game/_MAIN/zombie/bp_zombie.bp_zombie_C" (`self.Spawn LOCATION2`) "Undefined" "OverrideRootScale" null null))
  (for _ (range 1 (+ (/ (`self.ZOMBIETOTAL`) 2) 1))
    (`|SpawnActorFromClass` "/Game/_MAIN/zombie/bp_zombie.bp_zombie_C" (`self.Spawn LOCATION3`) "Undefined" "OverrideRootScale" null null))
  (for _ (range 1 (+ (/ (`self.ZOMBIETOTAL`) 2) 1))
    (`|SpawnActorFromClass` "/Game/_MAIN/zombie/bp_zombie.bp_zombie_C" (`self.spawn location4`) "Undefined" "OverrideRootScale" null null)))

(event `WAVE INCREAMENT`
  ;[1 1 1] wave
  (if (== (`self.CURRENT WAVE`) (`self.MAXWAVES`))
    (`self.player wins`)
    (else
      (`/Engine/EditorBlueprintResources/StandardMacros.IncrementInt` (`self.CURRENT WAVE`)
        (:`  `
          (`self.WAVE START`))))))

(event `player wins`
  ;[1 1 1] win
  (bind _asbp_first_person_character (cast `/Game/_MAIN/BLUEPRINTS/BP_FirstPersonCharacter` (`GameplayStatics.GetPlayerCharacter` 0)))
  (`/Game/_MAIN/BLUEPRINTS/BP_FirstPersonCharacter.showwinui` _asbp_first_person_character))

(fn `UserConstructionScript`)